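; Behavior tree task that selects the next patrol waypoint for an NPC.
; It reads PatrolPoints from the controlled ThirdPersonCharacter and writes the entry at the blackboard Index to NextWaypoint.
; It then increments Index modulo the array length, so the route loops, and finishes successfully.
; A failed cast stops execution without calling FinishExecute.
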(event EventReceiveExecuteAI
  (params (OwnerController :type AI%20Controller%20Object%20Reference) (ControlledPawn :type Pawn%20Object%20Reference))
  (bind _index (Variables|Default|GetIndex))
  (bind _returnvalue (Class|BTFunctionLibrary|GetBlackboardValueasInt _index))
  (bind _asthird_person_character (Utilities|Casting|CastToThirdPersonCharacter ControlledPawn))
  (bind _output_get (Variables|Default|SetPatrol%20Points (Variables|/Game/Trash/ThirdPersonCharacter.ThirdPersonCharacter_C|GetPatrolPoints _asthird_person_character)))
  (Class|BTFunctionLibrary|SetBlackboardValueasObject (Variables|Default|GetNextWaypoint) (Utilities|Array|Get(acopy) _output_get _returnvalue))
  (Class|BTFunctionLibrary|SetBlackboardValueasInt (Variables|Default|GetIndex) (Math|Integer|%(Integer) (+ _returnvalue 1) (Utilities|Array|Length _output_get)))
  (AI|BehaviorTree|FinishExecute true))