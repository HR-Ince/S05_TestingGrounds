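; AI controller for guard NPCs that patrol and shoot at the player.
; On begin play it sets up the PatrolData blackboard and runs the GuardBehaviour behavior tree.
; Perception updates set the Enemy blackboard key when a living, player-controlled TPCharacter is sensed, and clear it otherwise.
; Each tick, the controlled character's Aiming and Shooting flags mirror whether Enemy is valid.
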(event OnTargetPerceptionUpdated(AIPerception)
  (params (Actor :type Actor%20Object%20Reference) (Stimulus :type AI%20Stimulus%20Structure))
  (bind _returnvalue (Pawn|GetControlledPawn))
  (bind _returnvalue_2 (Utilities|String|StringToName "Enemy"))
  (bind _returnvalue_3 (AI|GetBlackboard _returnvalue))
  (bind _astpcharacter (Utilities|Casting|CastToTPCharacter Actor))
  (bind _worthshooting (CallFunction|CheckWorthShooting _astpcharacter Stimulus))
  (if _worthshooting
    (AI|Components|Blackboard|SetValueasObject _returnvalue_3 _returnvalue_2 _astpcharacter)
    (else
      (AI|Components|Blackboard|ClearValue _returnvalue_3 _returnvalue_2))))

(event EventBeginPlay
  (Class|AIController|UseBlackboard "/Game/Dynamic/NPCs/AI/PatrolData.PatrolData")
  (AI|RunBehaviorTree "/Game/Dynamic/NPCs/AI/GuardBehaviour.GuardBehaviour"))

(event EventTick
  (params (DeltaSeconds :type Float%20%28single-precision%29))
  (bind _astpcharacter (Utilities|Casting|CastToTPCharacter (Pawn|GetControlledPawn)))
  (bind _output_get (Variables|/Game/Dynamic/NPCs/Behaviour/TPCharacter.TPCharacter_C|SetAiming _astpcharacter (Utilities|IsValid (AI|Components|Blackboard|GetValueasObject (AI|GetBlackboard _astpcharacter) (Utilities|String|StringToName "Enemy")))))
  (Variables|/Game/Dynamic/NPCs/Behaviour/TPCharacter.TPCharacter_C|SetShooting _astpcharacter _output_get))

(fn ConstructionScript)

(fn CheckWorthShooting
  (params (Target :type TP%20Character%20Object%20Reference) (Stimulus :type AI%20Stimulus%20Structure))
  (bind _dead (Default|IsDead Target))
  (return (Math|Boolean|ANDBoolean (not _dead) (Pawn|IsPlayerControlled Target) (.bSuccessfullySensed (Utilities|Struct|BreakAIStimulus Stimulus)))))