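; NPC_AI_BP is an AI controller for guard NPCs that tracks the player's first-person character.
; On BeginPlay it initializes the PatrolData blackboard and runs the GuardBehaviour behavior tree.
; AI Perception updates write the sensed character to the blackboard's Enemy key and clear it when sensing is lost, ignoring other actor types.
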(event OnTargetPerceptionUpdated(AIPerception)
  (params (Actor :type Actor%20Object%20Reference) (Stimulus :type AI%20Stimulus%20Structure))
  (bind _returnvalue (Pawn|GetControlledPawn))
  (bind _returnvalue_2 (Utilities|String|StringToName "Enemy"))
  (bind _returnvalue_3 (AI|GetBlackboard _returnvalue))
  (bind _asfirst_person_character (Utilities|Casting|CastToFirstPersonCharacter Actor))
  (if (.bSuccessfullySensed (Utilities|Struct|BreakAIStimulus Stimulus))
    (AI|Components|Blackboard|SetValueasObject _returnvalue_3 _returnvalue_2 _asfirst_person_character)
    (else
      (AI|Components|Blackboard|ClearValue _returnvalue_3 _returnvalue_2))))

(event EventBeginPlay
  (Class|AIController|UseBlackboard "/Game/Static/NPCs/AI/PatrolData.PatrolData")
  (AI|RunBehaviorTree "/Game/Static/NPCs/AI/GuardBehaviour.GuardBehaviour"))

(fn ConstructionScript)